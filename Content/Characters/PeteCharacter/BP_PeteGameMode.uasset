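; Game mode for the Pete character levels that sets up the lives HUD and starts level progression.
; On BeginPlay it adds the WBP_Lives widget, then calls BeginNextLevel on BP_GameInstance with the player character.
; ShowEndScreen adds the WBP_EndScreen widget, shows the mouse cursor and returns the widget to the caller.
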(event `self.ReceiveBeginPlay`
  (bind _returnvalue (`|CreateWidget` "/Game/UI/WBP_Lives.WBP_Lives_C"))
  (`UserWidget.AddToViewport` _returnvalue 0)
  (bind _asbp_game_instance (cast `/Game/GameInstance/BP_GameInstance` (`GameplayStatics.GetGameInstance`)))
  (`/Game/GameInstance/BP_GameInstance.BeginNextLevel` _asbp_game_instance (`GameplayStatics.GetPlayerCharacter` 0)))

(fn `ShowEndScreen`
  (returns (EndScreenWidget :type "/Game/UI/WBP_EndScreen Object Reference"))
  (bind _returnvalue (`|CreateWidget` "/Game/UI/WBP_EndScreen.WBP_EndScreen_C"))
  (`UserWidget.AddToViewport` _returnvalue 0)
  (set `PlayerController.bShowMouseCursor` true (`GameplayStatics.GetPlayerController` 0))
  (return _returnvalue))

(fn `UserConstructionScript`)