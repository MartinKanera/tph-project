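; AI controller for the maze guard that wanders between random navmesh points and heads for the player when perceived.
; AI perception updates send the guard to the player's current position.
; Tick picks a new nearby point on arrival (2D distance check), and a looping timer re-rolls the target to unstick it.
; All moves share MoveToRandomLocation, which draws a debug sphere; the Behavior Tree and Blackboard nodes never run.
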(event `self.ReceivePossess`
  (params (PossessedPawn :type "Pawn Object Reference"))
  ;[1 1 1] 2. Set Random Target Location
  (`self.MoveToRandomLocation` (`self.K2_GetActorLocation` (`self.K2_GetPawn`)) 1500.0))

(event `self.ReceiveBeginPlay`
  ;[1 1 1] Setup Events
  (add `AIPerceptionComponent.OnPerceptionUpdated` (`self.AIPerception`) (delegate `OnPerceptionUpdated_Event`))
  (`KismetSystemLibrary.K2_SetTimerDelegate` (delegate `Update Target Location`) 20.0 true false 0.0 5.0))

(event `OnPerceptionUpdated_Event`
  (params (UpdatedActors :type "Array of Actor Object Reference (by ref)"))
  ;[1 1 1] Move Target Location to Player Position
  (for _array_element UpdatedActors
    (bind _asbp_third_person_character (cast `/Game/Characters/PeteCharacter/BP_ThirdPersonCharacter` _array_element))
    (bind _output_get (set `self.TargetLocation` (`self.K2_GetActorLocation` _asbp_third_person_character)))
    ;[1 1 1] Approach the player
    (`self.MoveToRandomLocation` _output_get)))

(event `Update Target Location`
  ;[1 1 1] Unstuck Guard
  (`self.MoveToRandomLocation` (`self.TargetLocation`) 1500.0))

(event `self.ReceiveTick`
  (params (DeltaSeconds :type "Float (single-precision)"))
  ;[1 1 1] Is Guard At Target Location?
  (bind _returnvalue (`self.IsAtLocation` 50.0))
  (if _returnvalue
    ;[1 1 1] Move to Random Location
    (`self.MoveToRandomLocation` (`self.TargetLocation`) 1000.0)))

(fn `IsAtLocation`
  (params (toleranceRadius :type "Float (double-precision)"))
  (returns (ReturnValue :type Boolean))
  (return (<= (`KismetMathLibrary.VSize` (- (`KismetMathLibrary.MakeVector2D` (.x (`self.K2_GetActorLocation` (`self.K2_GetPawn`))) (.y (`self.K2_GetActorLocation` (`self.K2_GetPawn`)))) (`KismetMathLibrary.MakeVector2D` (.x (`self.TargetLocation`)) (.y (`self.TargetLocation`))))) (`local.toleranceRadius`))))

(fn `MoveToRandomLocation`
  (params (Origin :type "Vector Structure (by ref)") (Radius :type "Float (double-precision)"))
  (bind _randomlocation (`NavigationSystemV1.K2_GetRandomLocationInNavigableRadius` Origin Radius null null))
  (bind _output_get (set `self.TargetLocation` (`KismetMathLibrary.MakeVector` (.x _randomlocation) (.y _randomlocation) (.z (`self.K2_GetActorLocation` (`self.K2_GetPawn`))))))
  (`self.MoveToLocation` _output_get 5.0 true true false true null)
  (`KismetSystemLibrary.DrawDebugSphere` _output_get 50.0 12 (struct :`R` 1.0 :`G` 1.0 :`B` 1.0 :`A` 1.0) 5.0))

(fn `UserConstructionScript`)