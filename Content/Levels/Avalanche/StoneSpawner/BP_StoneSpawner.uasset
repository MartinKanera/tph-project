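; BP_StoneSpawner is a spawner in the Avalanche level that releases rocks at random intervals for as long as it runs.
; From BeginPlay, SpawnStone pushes the previous rock with a fixed world-space impulse and waits briefly.
; It then spawns a new BP_Rock at SpawnPoint, stores it as CurrentRock and re-arms itself through a randomized function-name timer, so each rock rests until the next cycle.
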(event `SpawnStone`
  (`self.PushRock`
    (:` `
      (bind _returnvalue (`|SpawnActorFromClass` "/Game/Levels/Avalanche/Rock/BP_Rock.BP_Rock_C" (`SceneComponent.K2_GetComponentToWorld` (`self.SpawnPoint`)) "AdjustIfPossibleButAlwaysSpawn" "MultiplyWithRoot" null null))
      (set `self.CurrentRock` _returnvalue)
      (`self.SpawnStoneTimer`))))

(event `self.ReceiveBeginPlay`
  (`self.BeginSpawningLoop`))

(event `BeginSpawningLoop`
  (`self.SpawnStone`)
  (`self.SpawnStoneTimer`))

(fn `UserConstructionScript`)