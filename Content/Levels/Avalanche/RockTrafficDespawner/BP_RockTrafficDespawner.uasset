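; Avalanche level actor that destroys boulders (BP_Rock) that linger inside its box volume longer than DestroyDelay, apparently to clear rock traffic jams.
; Box overlap events record each entering rock with a timestamp in OverlappingRocks and drop it when it leaves.
; StartValidatingRocks runs a looping one-second timer that destroys expired rocks, and StopValidatingRocks clears that timer.
; The RemoveExpiredRocks function is an empty stub.
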(event `StopValidatingRocks`
  (`KismetSystemLibrary.K2_ClearAndInvalidateTimerHandle` (`self.CurrentTimerHandle`)))

(event `StartValidatingRocks`
  (bind _returnvalue (`KismetSystemLibrary.K2_SetTimerDelegate` (delegate `DespawnExpiredRocks`) 1.0 true true))
  (set `self.CurrentTimerHandle` _returnvalue))

(event `DespawnExpiredRocks`
  (for _array_element (`self.OverlappingRocks`)
    (if (> (- (`KismetSystemLibrary.GetGameTimeInSeconds`) (`.Timestamp_5_635A80F9FE457C3ADEE7CAA0D8AEA88D` (break `/Game/Levels/Avalanche/RockTrafficDespawner/FStruct_BoulderData` _array_element))) (`self.DestroyDelay`))
      (`self.K2_DestroyActor` (break `/Game/Levels/Avalanche/RockTrafficDespawner/FStruct_BoulderData` _array_element)))))

(event `self.Box.OnComponentBeginOverlap`
  (params (OverlappedComponent :type "PrimitiveComponent Object Reference") (OtherActor :type "Actor Object Reference") (OtherComp :type "PrimitiveComponent Object Reference") (OtherBodyIndex :type Integer) (bFromSweep :type Boolean) (SweepResult :type "HitResult Structure (by ref)"))
  (bind _asbp_rock (cast `/Game/Levels/Avalanche/Rock/BP_Rock` OtherActor))
  (`KismetArrayLibrary.Array_Add` (`self.OverlappingRocks`) (make `/Game/Levels/Avalanche/RockTrafficDespawner/FStruct_BoulderData` _asbp_rock (`KismetSystemLibrary.GetGameTimeInSeconds`))))

(event `self.Box.OnComponentEndOverlap`
  (params (OverlappedComponent :type "PrimitiveComponent Object Reference") (OtherActor :type "Actor Object Reference") (OtherComp :type "PrimitiveComponent Object Reference") (OtherBodyIndex :type Integer))
  (bind _asbp_rock (cast `/Game/Levels/Avalanche/Rock/BP_Rock` OtherActor))
  (for (_array_element _array_index) (`self.OverlappingRocks`)
    (if (== (break `/Game/Levels/Avalanche/RockTrafficDespawner/FStruct_BoulderData` _array_element) _asbp_rock)
      (`KismetArrayLibrary.Array_Remove` (`self.OverlappingRocks`) _array_index)
      (break))))

(fn `RemoveExpiredRocks`)

(fn `UserConstructionScript`)