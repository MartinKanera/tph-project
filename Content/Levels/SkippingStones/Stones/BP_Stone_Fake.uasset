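; BP_Stone_Fake is a decoy stone in the Skipping Stones level that sinks while something overlaps it.
; Overlapping its sphere plays a comic splash sound and runs the Sink timeline, offsetting the mesh's Z from its starting height.
; Ending the overlap reverses the timeline to float the stone back up.
; The timeline update feeds the mesh's world X and Y into its relative location.
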(event `self.ReceiveBeginPlay`
  (bind (_relativelocation_x _relativelocation_y _relativelocation_z) (`KismetMathLibrary.BreakVector` (`SceneComponent.RelativeLocation` (`self.SM_Stone`))))
  (set `self.InitialZ` _relativelocation_z))

(event `SinkStone`
  (bind _sm_stone (`self.SM_Stone`))
  (bind (_returnvalue_x _returnvalue_y) (`KismetMathLibrary.BreakVector` (`SceneComponent.K2_GetComponentLocation` _sm_stone)))
  (bind (_direction _progress) (`Timeline|Sink` :!label _label)
    (:`Update`
      (`SceneComponent.K2_SetRelativeLocation` _sm_stone (`KismetMathLibrary.MakeVector` _returnvalue_x _returnvalue_y (+ (`self.InitialZ`) (* _progress (`self.SinkZOffset`)))) false false))))

(event `FloatStone`
  (goto _label :!via `Reverse`))

(event `self.Sphere.OnComponentBeginOverlap`
  (params (OverlappedComponent :type "PrimitiveComponent Object Reference") (OtherActor :type "Actor Object Reference") (OtherComp :type "PrimitiveComponent Object Reference") (OtherBodyIndex :type Integer) (bFromSweep :type Boolean) (SweepResult :type "HitResult Structure (by ref)"))
  (`GameplayStatics.SpawnSoundAtLocation` "/Game/Audio/Sfx/Splash/SC_SplashFunny.SC_SplashFunny" (`SceneComponent.K2_GetComponentLocation` OverlappedComponent) (struct) 1.0 1.0 0.0 "/Game/Audio/SA_Low.SA_Low" null)
  (`self.SinkStone`))

(event `self.Sphere.OnComponentEndOverlap`
  (params (OverlappedComponent :type "PrimitiveComponent Object Reference") (OtherActor :type "Actor Object Reference") (OtherComp :type "PrimitiveComponent Object Reference") (OtherBodyIndex :type Integer))
  (`self.FloatStone`))

(fn `UserConstructionScript`)