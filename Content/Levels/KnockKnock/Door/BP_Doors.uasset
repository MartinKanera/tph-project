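; Double door Blueprint in the KnockKnock level that swings open when something overlaps its trigger, if it is openable.
; On overlap, the IsOpenable flag selects between opening the doors with a large door sound and playing only a gong.
; OpenDoor plays a timeline that yaws the right and left panels in opposite directions up to a quarter turn.
; Sounds play at the overlapping component's location, and there is no closing logic.
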(event `OpenDoor`
  (bind (_direction _opendoortrack) (`Timeline|Timeline`)
    (:`Update`
      (bind _returnvalue (* _opendoortrack 90.0))
      (`SceneComponent.K2_SetRelativeRotation` (`self.DoorRight`) (`KismetMathLibrary.MakeRotator` 0.0 0.0 _returnvalue) false false)
      (`SceneComponent.K2_SetRelativeRotation` (`self.DoorLeft`) (`KismetMathLibrary.MakeRotator` 0.0 0.0 (* _returnvalue -1.0)) false false))))

(event `self.CollisionTrigger.OnComponentBeginOverlap`
  (params (OverlappedComponent :type "PrimitiveComponent Object Reference") (OtherActor :type "Actor Object Reference") (OtherComp :type "PrimitiveComponent Object Reference") (OtherBodyIndex :type Integer) (bFromSweep :type Boolean) (SweepResult :type "HitResult Structure (by ref)"))
  (bind _returnvalue (`SceneComponent.K2_GetComponentLocation` OtherComp))
  (if (`self.bIsOpenable`)
    (`self.OpenDoor`)
    (`GameplayStatics.PlaySoundAtLocation` "/Game/Audio/Sfx/Door/SC_LargeDoor.SC_LargeDoor" _returnvalue (struct) 1.0 1.0 0.0 "/Game/Audio/SA_Low.SA_Low" null null null)
    (else
      (`GameplayStatics.PlaySoundAtLocation` "/Game/Audio/Sfx/Gong/SC_Gong.SC_Gong" _returnvalue (struct) 1.0 1.0 0.0 "/Game/Audio/SA_Low.SA_Low" null null null))))

(fn `UserConstructionScript`)